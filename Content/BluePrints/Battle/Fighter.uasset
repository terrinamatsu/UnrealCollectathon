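; Fighter actor for battles, representing one creature of a given Specie with gender and optional nickname.
; On construction it rolls gender against the species' PercentageMale, with 101 meaning genderless, though it sets Specie to None just before reading it.
; GetName returns the nickname while its flag is set, otherwise the species name.
; DecreaseHealth is an empty stub and the event graph holds only disabled default events.
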(event EventBeginPlay)

(event Collision|EventActorBeginOverlap
  (params (OtherActor :type Actor%20Object%20Reference)))

(event EventTick
  (params (DeltaSeconds :type Float%20%28single-precision%29)))

(fn ConstructionScript
  (CallFunction|DetermineGender))

(fn DetermineGender
  (bind _output_get (Variables|Default|Setspecie 0))
  (if (== (Variables|/Game/BluePrints/Battle/Specie.Specie_C|GetpercentageMale _output_get) 101)
    (Variables|Default|Setgender "N")
    (elif (>= (Variables|/Game/BluePrints/Battle/Specie.Specie_C|GetpercentageMale _output_get) (Math|Random|RandomInteger 100))
      (Variables|Default|Setgender "M")
      (else
        (Variables|Default|Setgender "F")))))

(fn ChangeNickname
  (params (newName :type String))
  (Variables|Default|SetnickName newName)
  (Variables|Default|SetnickNameFlag true))

(fn DecreaseHealth)

(fn RemoveNickname
  (Variables|Default|SetnickNameFlag false))

(fn GetName
  (if (Variables|Default|GetnickNameFlag)
    (return (Variables|Default|GetnickName))
    (else
      (return (Variables|/Game/BluePrints/Battle/Specie.Specie_C|GetspecieName (Variables|Default|Getspecie))))))