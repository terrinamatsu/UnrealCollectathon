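; BP_HouseCamTest is a trigger-volume camera that takes over the view while the third-person character is inside its cylinder.
; On overlap it swaps the character's follow camera for its own, sets the character's IsCameraLocked flag and switches the player's view target to itself.
; Leaving the cylinder reverses this, returning the view to the pawn.
; Every tick the camera rotates to look at the player pawn.
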(event OnComponentBeginOverlap(Cylinder)
  (params (OverlappedComponent :type Primitive%20Component%20Object%20Reference) (OtherActor :type Actor%20Object%20Reference) (OtherComp :type Primitive%20Component%20Object%20Reference) (OtherBodyIndex :type Integer) (bFromSweep :type Boolean) (SweepResult :type Hit%20Result%20Structure%20%28by%20ref%29))
  (bind _asthird_person_character (Utilities|Casting|CastToThirdPersonCharacter OtherActor))
  (Components|Activation|SetActive (Variables|/Game/ThirdPersonBP/Blueprints/ThirdPersonCharacter.ThirdPersonCharacter_C|GetFollowCamera _asthird_person_character) false false)
  (Variables|/Game/ThirdPersonBP/Blueprints/ThirdPersonCharacter.ThirdPersonCharacter_C|SetisCameraLocked _asthird_person_character true)
  (Components|Activation|SetActive (Variables|Default|GetCamera) true true)
  (Game|Player|SetViewTargetwithBlend (Game|GetPlayerController 0) self 0.0 "VTBlend_Linear" 0.0 false))

(event OnComponentEndOverlap(Cylinder)
  (params (OverlappedComponent :type Primitive%20Component%20Object%20Reference) (OtherActor :type Actor%20Object%20Reference) (OtherComp :type Primitive%20Component%20Object%20Reference) (OtherBodyIndex :type Integer))
  (bind _asthird_person_character (Utilities|Casting|CastToThirdPersonCharacter OtherActor))
  (Components|Activation|SetActive (Variables|/Game/ThirdPersonBP/Blueprints/ThirdPersonCharacter.ThirdPersonCharacter_C|GetFollowCamera _asthird_person_character) true false)
  (Variables|/Game/ThirdPersonBP/Blueprints/ThirdPersonCharacter.ThirdPersonCharacter_C|SetisCameraLocked _asthird_person_character false)
  (Components|Activation|SetActive (Variables|Default|GetCamera) false true)
  (Game|Player|SetViewTargetwithBlend (Game|GetPlayerController 0) (Game|Player|GetPlayerPawn 0) 0.0 "VTBlend_Linear" 0.0 false))

(event EventBeginPlay)

(event Collision|EventActorBeginOverlap
  (params (OtherActor :type Actor%20Object%20Reference)))

(event EventTick
  (params (DeltaSeconds :type Float%20%28single-precision%29))
  (bind _camera (Variables|Default|GetCamera))
  (Transformation|SetWorldRotation _camera (Math|Rotator|FindLookatRotation (Transformation|GetWorldLocation _camera) (Transformation|GetActorLocation (Game|Player|GetPlayerPawn 0))) false false))

(fn ConstructionScript)