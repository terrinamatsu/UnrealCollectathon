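; NPC Blueprint that offers speech to the player's ThirdPersonCharacter while it overlaps the actor.
; On overlap begin it flags speech as available and copies its NPCImage and Speech onto the character; on overlap end it clears the speech flags.
; A C-key FlipFlop calls a one-second view-target blend on its A branch only, with no target specified.
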(event EventBeginPlay)

(event Collision|EventActorBeginOverlap
  (params (OtherActor :type Actor%20Object%20Reference))
  (bind _asthird_person_character (Utilities|Casting|CastToThirdPersonCharacter OtherActor))
  (Variables|/Game/ThirdPersonBP/Blueprints/ThirdPersonCharacter.ThirdPersonCharacter_C|SetisSpeechAvailable _asthird_person_character true)
  (Variables|/Game/ThirdPersonBP/Blueprints/ThirdPersonCharacter.ThirdPersonCharacter_C|SetisSpeech _asthird_person_character false)
  (Variables|/Game/ThirdPersonBP/Blueprints/ThirdPersonCharacter.ThirdPersonCharacter_C|SetCurrentNPC_Image _asthird_person_character (Variables|Default|GetNPC_Image))
  (Variables|/Game/ThirdPersonBP/Blueprints/ThirdPersonCharacter.ThirdPersonCharacter_C|SetCurrentSpeech _asthird_person_character (Variables|Default|Getspeech)))

(event EventTick
  (params (DeltaSeconds :type Float%20%28single-precision%29)))

(event Collision|EventActorEndOverlap
  (params (OtherActor :type Actor%20Object%20Reference))
  (bind _asthird_person_character (Utilities|Casting|CastToThirdPersonCharacter OtherActor))
  (Variables|/Game/ThirdPersonBP/Blueprints/ThirdPersonCharacter.ThirdPersonCharacter_C|SetisSpeechAvailable _asthird_person_character false)
  (Variables|/Game/ThirdPersonBP/Blueprints/ThirdPersonCharacter.ThirdPersonCharacter_C|SetisSpeech _asthird_person_character false))

(event Input|KeyboardEvents|C
  (params (Key :type Key%20Structure))
  (:Pressed
    (Utilities|FlowControl|FlipFlop
      (:A
        (Game|Player|SetViewTargetwithBlend (Game|GetPlayerController 0) 0 1.0 "VTBlend_Linear" 0.0 false)))))

(fn ConstructionScript)