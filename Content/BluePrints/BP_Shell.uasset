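; BP_Shell is a collectable shell that the ThirdPersonCharacter picks up by overlapping it.
; A one-time IsCollected guard gates the pickup, which toggles the shell mesh and CollectableGetEffect visibility and plays a rupee sound.
; After a short delay it scales the Box to zero instead of destroying the actor.
; BeginPlay casts the ShellNo widget to HUD but does nothing with it, and no count is updated here.
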(event EventBeginPlay
  (Utilities|Casting|CastToHUD (UserInterface|GetUserWidgetObject (Variables|Default|GetshellNo))))

(event EventTick
  (params (DeltaSeconds :type Float%20%28single-precision%29)))

(event Collision|EventActorBeginOverlap
  (params (OtherActor :type Actor%20Object%20Reference))
  ;[1 1 1] collected
  (Utilities|Casting|CastToThirdPersonCharacter OtherActor)
  (if (not (Variables|Default|GetIsCollected))
    (Variables|Default|SetIsCollected true)
    (Rendering|ToggleVisibility (Variables|Default|Getshell) false)
    (Rendering|ToggleVisibility (Variables|Default|GetCollectableGetEffect) false)
    (Audio|PlaySoundatLocation "/Game/Sounds/SFXNON/OOT_Get_Rupee.OOT_Get_Rupee" (Transformation|GetActorLocation) "0, 0, 0" 1.0 1.0 0.0 0 0 0)
    (Utilities|FlowControl|Delay 0.5)
    (Transformation|SetWorldScale3D (Variables|Default|GetBox) "0, 0, 0")))

(fn ConstructionScript
  (Rendering|ToggleVisibility (Variables|Default|GetCollectableGetEffect) false))