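; Order chest for a sequence puzzle that the player solves by touching chests in numerical order.
; On box overlap it compares its OrderNum to the ThirdPersonCharacter's CurrentChest: a match advances the count, skipping ahead resets it to 1, and earlier chests do nothing.
; A match flashes the number and a skip flashes an error text, using delayed visibility toggles.
; A correct FinalCheck chest toggles the gem's visibility instead of advancing.
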(event OnComponentBeginOverlap(Box)
  (params (OverlappedComponent :type Primitive%20Component%20Object%20Reference) (OtherActor :type Actor%20Object%20Reference) (OtherComp :type Primitive%20Component%20Object%20Reference) (OtherBodyIndex :type Integer) (bFromSweep :type Boolean) (SweepResult :type Hit%20Result%20Structure%20%28by%20ref%29))
  (bind _ordernum (Variables|Default|GetorderNum))
  (bind _textrender (Variables|Default|GetTextRender))
  (bind _textrender_2 (Variables|Default|GetTextRender))
  (bind _asthird_person_character (Utilities|Casting|CastToThirdPersonCharacter OtherActor))
  (if (== (Variables|/Game/ThirdPersonBP/Blueprints/ThirdPersonCharacter.ThirdPersonCharacter_C|GetcurrentChest _asthird_person_character) _ordernum)
    (Rendering|Components|TextRender|SetText _textrender (Utilities|Text|ToText(Integer) (Variables|Default|GetorderNum)))
    (Rendering|ToggleVisibility _textrender false)
    (if (Math|Boolean|Equal(Boolean) (Variables|Default|GetfinalCheck) true)
      (Utilities|FlowControl|Delay 0.2)
      (Rendering|ToggleVisibility _textrender false)
      (Rendering|ToggleVisibility (Variables|Default|GetBP_Gem) false)
      (else
        (Variables|/Game/ThirdPersonBP/Blueprints/ThirdPersonCharacter.ThirdPersonCharacter_C|SetcurrentChest _asthird_person_character (+ _ordernum 1))
        (Utilities|FlowControl|Delay 0.2)
        (Rendering|ToggleVisibility (Variables|Default|GetTextRender) false)))
    (elif (not (> (Variables|/Game/ThirdPersonBP/Blueprints/ThirdPersonCharacter.ThirdPersonCharacter_C|GetcurrentChest _asthird_person_character) _ordernum))
      (Variables|/Game/ThirdPersonBP/Blueprints/ThirdPersonCharacter.ThirdPersonCharacter_C|SetcurrentChest _asthird_person_character 1)
      (Rendering|Components|TextRender|SetText _textrender (Variables|Default|GetX))
      (Rendering|ToggleVisibility _textrender_2 false)
      (Utilities|FlowControl|Delay 0.2)
      (Rendering|ToggleVisibility _textrender_2 false))))

(event EventBeginPlay)

(event Collision|EventActorBeginOverlap
  (params (OtherActor :type Actor%20Object%20Reference)))

(event EventTick
  (params (DeltaSeconds :type Float%20%28single-precision%29)))

(fn ConstructionScript
  (Rendering|ToggleVisibility (Variables|Default|GetTextRender) false)
  (Rendering|ToggleVisibility (Variables|Default|GetBP_Gem) false))